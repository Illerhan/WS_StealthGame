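; Base enemy character that supplies attack, weapon, patrol route and movement-speed actions.
; Attack plays a pistol montage and fires OnAttackEnd whether it completes or is interrupted.
; WieldWeapon spawns a BP_Gun, snaps it to a mesh socket and sets the IsWealdingSword flag, despite the gun.
; SetMouvementSpeed maps a speed state to max walk speed, GetPatrolRoute exposes the assigned route, and OnLoos is empty.
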(event Custom|WieldWeapon
  (bind _returnvalue (Game|SpawnActorfromClass "/Game/Thomas_A/BP/BP_Gun.BP_Gun_C" (Transformation|GetActorTransform) "Undefined" "MultiplyWithRoot" 0 0))
  (Transformation|AttachComponentToComponent _returnvalue (Variables|Character|GetMesh) "Weapon_L" "SnapToTarget" "SnapToTarget" "SnapToTarget" true)
  (Variables|Default|SetisWealdingSword true))

(event Custom|Attack
  (Animation|Montage|PlayMontage (Variables|Character|GetMesh) "/Game/Ennemy/Animation/Montage_Pistol.Montage_Pistol" 0.75
    (:OnCompleted
      _)
    (:OnInterrupted
      _))
  (Default|CallOnAttackEnd))

(event EventBeginPlay)

(event Collision|EventActorBeginOverlap
  (params (OtherActor :type Actor%20Object%20Reference)))

(fn ConstructionScript
  (|CallParentFunction))

(fn OnLoos)

(fn GetPatrolRoute
  (return (Variables|AI|GetPatrolRoute)))

(fn SetMouvementSpeed
  (params (Speed :type E_MouvementSpeed%20Enum :default "NewEnumerator0"))
  (bind _output_get (Variables|/Script/Engine.CharacterMovementComponent|SetMaxWalkSpeed (Variables|Character|GetCharacterMovement) (Utilities|Select :Index Speed :NewEnumerator0 0.0 :NewEnumerator1 1e+02 :NewEnumerator2 3e+02 :NewEnumerator3 5e+02)))
  (return _output_get))